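; A bullet projectile actor that bounces off surfaces and removes itself after a short lifetime set on BeginPlay.
; The construction script configures ProjectileMovement to move the Sphere component, taking initial and max speed from MoveSpeed and enabling bounce.
; Commented, unconnected EventGraph examples show alternative timed-destruction techniques: Delay, accumulated time and a timer by function name.
; The timer's AutoDestroy target only prints a message, with its DestroyActor node disconnected.
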(event `self.ReceiveBeginPlay`
  ;[1 1 1] 자동으로 자신을 파괴하는 기능
  ;;[1 0.1719 0.1719] BeginPlay -> 액터의 기본기능( 단순히 생명 시간 설정)
  (`self.SetLifeSpan` 2.0))

(event `self.ReceiveTick`
  (params (DeltaSeconds :type "Float (single-precision)")))

(fn `AutoDestroy`
  (`KismetSystemLibrary.PrintString` "Hello"))

(fn `UserConstructionScript`
  (set `ProjectileMovementComponent.InitialSpeed` (`self.MoveSpeed`) (`self.ProjectileMovement`))
  (set `ProjectileMovementComponent.MaxSpeed` (`self.MoveSpeed`) (`self.ProjectileMovement`))
  (set `ProjectileMovementComponent.Bounciness` 0.6 (`self.ProjectileMovement`))
  (set `ProjectileMovementComponent.bShouldBounce` true (`self.ProjectileMovement`))
  (`MovementComponent.SetUpdatedComponent` (`self.ProjectileMovement`) (`self.Sphere`)))