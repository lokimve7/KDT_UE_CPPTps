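; Enemy manager actor meant to periodically spawn BP_Only_Enemy at random spawn points in the level.
; BeginPlay caches every actor with "BP_Spawn" in its display name and starts a looping timer on CreateEnemy, which is empty.
; Spawning lives in Tick, gated by CurrTime exceeding CreateTime, but CurrTime adds zero each frame rather than delta time, so it never advances.
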(event `self.ReceiveBeginPlay`
  (bind _outactors (`GameplayStatics.GetAllActorsOfClass` "/Script/Engine.Actor"))
  (for _array_element _outactors
    (if (`KismetStringLibrary.Contains` (`KismetSystemLibrary.GetDisplayName` _array_element) "BP_Spawn")
      (`KismetArrayLibrary.Array_Add` (`self.allSpanwPos`) _array_element)))
  (`KismetSystemLibrary.K2_SetTimerDelegate` (delegate `CreateEnemy`) 2.0 true))

(event `CreateEnemy`)

(event `self.ReceiveTick`
  (params (DeltaSeconds :type "Float (single-precision)"))
  (bind _output_get (set `self.currTime` (+ 0.0 (`self.currTime`))))
  (if (> _output_get (`self.createTime`))
    (`|SpawnActorFromClass` "/Game/Blueprints/OnlyBlueprints/BP_Only_Enemy.BP_Only_Enemy_C" (`KismetMathLibrary.MakeTransform` (`self.K2_GetActorLocation` (`|GetArrayItem` (`self.allSpanwPos`) (`KismetMathLibrary.RandomIntegerInRange` 0 (- (`KismetArrayLibrary.Array_Length` (`self.allSpanwPos`)) 1))))) "Undefined" "MultiplyWithRoot" null null)
    (set `self.currTime` 0.0)))

(fn `UserConstructionScript`)