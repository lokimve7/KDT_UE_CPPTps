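; BP_Only_TpsPlayer is a third-person player Blueprint that moves itself from horizontal and vertical input values.
; Each Tick, it weights the actor's right and forward vectors by those values and normalizes their sum into a direction.
; It then applies P = P0 + vt with MoveSpeed and delta time through SetActorLocation, without sweep, so movement does no collision check.
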(event `self.ReceiveTick`
  (params (DeltaSeconds :type "Float (single-precision)"))
  ;[1 1 1] P= P0 + vt
  (`self.K2_SetActorLocation` (+ (`self.K2_GetActorLocation`) (* DeltaSeconds (* (`KismetMathLibrary.Normal` (+ (* (`self.GetInputAxisValue`) (`self.GetActorRightVector`)) (* (`self.GetInputAxisValue`) (`self.GetActorForwardVector`)))) (`self.MoveSpeed`))))))

(fn `UserConstructionScript`)