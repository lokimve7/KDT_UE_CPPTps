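; Finite state machine component for BP_Only_Enemy that drives idle, chase, attack, attack delay, damage and death against the player.
; Tick dispatches per-state updates using distance checks and timers, chasing through AIController MoveToLocation.
; ChangeState centralizes transitions: it stops movement, resets the timer and syncs the Animation Blueprint state.
; It also picks random attack types, plays random hit or death montage sections, and disables capsule collision on death.
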(event `self.ReceiveBeginPlay`
  ;[1 1 1] 플레이어 찾자
  (bind _returnvalue (`GameplayStatics.GetActorOfClass` "/Game/Blueprints/OnlyBlueprints/BP_Only_TpsPlayer.BP_Only_TpsPlayer_C"))
  (set `self.target` _returnvalue)
  ;[1 1 1] 나의 액터를 찾자
  (bind _asbp_only_enemy (cast `/Game/Blueprints/OnlyBlueprints/BP_Only_Enemy` (`self.GetOwner`)))
  (set `self.myActor` _asbp_only_enemy)
  ;[1 1 1] 나의 Animation Blueprint 가져오자
  (bind _asabp_only_enemy (cast `/Game/Blueprints/OnlyBlueprints/ABP_Only_Enemy` (`SkeletalMeshComponent.GetAnimInstance` (`Character.Mesh` (`self.myActor`)))))
  (set `self.anim` _asabp_only_enemy)
  ;[1 1 1] AIController 를 가져오자
  (bind _asaicontroller (cast `AIController` (`Pawn.GetController` (`self.myActor`))))
  (set `self.ai` _asaicontroller))

(event `self.ReceiveTick`
  (params (DeltaSeconds :type "Float (single-precision)"))
  (`/Engine/EditorBlueprintResources/StandardMacros.IsValid` (`self.target`)
    (:`Is Valid`
      (switch `/Game/Blueprints/OnlyBlueprints/BP_Only_EnemyState` (`self.currState`)
        (:`NewEnumerator0`
          (`self.UpdateIdle`))
        (:`NewEnumerator1`
          (`self.UpdateMove`))
        (:`NewEnumerator2`
          (`self.UpdateAttack`))
        (:`NewEnumerator3`
          (`self.UpdateDamage`))
        (:`NewEnumerator5`
          (`self.UpdateAttackDelay`))))))

(fn `Change State`
  (params (state :type "/Game/Blueprints/OnlyBlueprints/BP_Only_EnemyState Enum" :default "NewEnumerator0"))
  (bind _myactor (`self.myActor`))
  (`KismetSystemLibrary.PrintString` (`KismetStringLibrary.Concat_StrStr` (`|GetEnumeratorNameAsString` (`self.currState`)) "---------->" (`|GetEnumeratorNameAsString` state)))
  (`Controller.StopMovement` (`self.ai`)) ; 네이게이션 동작 멈춰!
  (bind _output_get (set `self.currState` (`local.state`))) ; 현재 상태 갱신
  (bind _output_get_2 (set `/Game/Blueprints/OnlyBlueprints/ABP_Only_Enemy.state` _output_get (`self.anim`))) ; 애니메이션 상태 갱신
  (set `self.currTime` 0.0)
  (switch `/Game/Blueprints/OnlyBlueprints/BP_Only_EnemyState` _output_get_2
    (:`NewEnumerator2`
      ;[1 1 1] 랜덤한 공격 모션을 선택하자
      (set `/Game/Blueprints/OnlyBlueprints/ABP_Only_Enemy.attackType` (cast `/Game/Blueprints/OnlyBlueprints/BP_Only_AttackType` (`KismetMathLibrary.Conv_IntToByte` (`KismetMathLibrary.RandomIntegerInRange` 0 1))) (`self.anim`)))
    (:`NewEnumerator3`
      ;[1 1 1] 랜덤한 피격 모션 (Montage 이용)
      (`Character.PlayAnimMontage` (`self.myActor`) "/Game/Blueprints/OnlyBlueprints/EnemyMontage.EnemyMontage" 1.0 (`KismetStringLibrary.Conv_StringToName` (`KismetStringLibrary.Concat_StrStr` "Damage0" (`KismetStringLibrary.Conv_IntToString` (`KismetMathLibrary.RandomIntegerInRange` 1 2))))))
    (:`NewEnumerator4`
      ;[1 1 1] 죽음 상태 설정
      (`Character.PlayAnimMontage` _myactor "/Game/Blueprints/OnlyBlueprints/EnemyMontage.EnemyMontage" 1.0 "Die")
      (`PrimitiveComponent.SetCollisionEnabled` (`Character.CapsuleComponent` _myactor) "NoCollision"))))

(fn `UpdateAttack`
  (`self.Change State` "NewEnumerator5"))

(fn `UpdateAttackDelay`
  (bind _returnvalue (`KismetMathLibrary.Vector_Distance` (`Actor.K2_GetActorLocation` (`self.target`)) (`Actor.K2_GetActorLocation` (`self.myActor`))))
  ;[1 1 1] 시간을 흐르게 하자
  (bind _output_get (set `self.currTime` (+ (`self.currTime`) (`GameplayStatics.GetWorldDeltaSeconds`))))
  (if (> _output_get (`self.attackDelayTime`))
    (set `self.currTime` 0.0)
    ;[1 1 1] 만약에 Attack Range 플레어가 있다면 공격해라!!
    (if (< _returnvalue (`self.atttackRange`))
      (`self.Change State` "NewEnumerator2")
      (else
        ;[1 1 1] 그렇지않고 만약에 TraceRange 에 있다면 쫓아가라 (상태를 MOVE)
        (if (< _returnvalue (`self.traceRange`))
          (`self.Change State` "NewEnumerator1")
          (else
            ;[1 1 1] 그렇지 않으면 IDLE 상태로 가라
            (`self.Change State` "NewEnumerator0")))))))

(fn `UpdateDamage`
  (bind _output_get (set `self.currTime` (+ (`self.currTime`) (`GameplayStatics.GetWorldDeltaSeconds`))))
  (if (> _output_get (`self.damageDelayTime`))
    (`self.Change State` "NewEnumerator0")))

(fn `UpdateIdle`
  (if (< (`KismetMathLibrary.VSize` (- (`Actor.K2_GetActorLocation` (`self.target`)) (`Actor.K2_GetActorLocation` (`self.myActor`)))) (`self.traceRange`))
    (`self.Change State` "NewEnumerator1")))

(fn `UpdateMove`
  (locals (dir :type "Vector Structure") (dist :type "Float (double-precision)" :default 0.0))
  ;[1 1 1] 플레이어를 향하는 방향을 구하자  , 플레이어와의 거리가도 구하자
  (bind _output_get (set `local.dir` (- (`Actor.K2_GetActorLocation` (`self.target`)) (`Actor.K2_GetActorLocation` (`self.myActor`)))))
  (set `local.dist` (`KismetMathLibrary.VSize` _output_get))
  ;[1 1 1] Navigation 기능으로 목적지까지 가라
  (`AIController.MoveToLocation` (`self.ai`) (`Actor.K2_GetActorLocation` (`self.target`)) -1.0 true true false true null true)
  ;[1 1 1] 만약에 플레이어가 AttactRange 에 들어왔다면 ATTACK 상태로 바꿔라
  (if (< (`local.dist`) (`self.atttackRange`))
    (`self.Change State` "NewEnumerator2")))